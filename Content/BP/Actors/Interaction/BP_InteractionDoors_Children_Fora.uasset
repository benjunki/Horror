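; Interactive door child Blueprint that swings open or closed each time Interact fires.
; On opening, a dot product between the normalized player-to-door direction and the actor's forward vector records which side the player stands on.
; That sign picks a positive or negative 90-degree yaw, which the PortaAbrir timeline lerps onto the Door's relative rotation.
; Closing reverses the same timeline, reusing the stored side.
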(event `/Game/BP/Interface/BPI_Interaction.Interact`
  (if (`self.PortaAberta`)
    (set `self.PortaAberta` false)
    (bind (_direction _alpha) (`Timeline|PortaAbrir` :!via `ReverseFromEnd` :!label _label)
      (:`Update`
        (`SceneComponent.K2_SetRelativeRotation` (`self.Door`) (`KismetMathLibrary.MakeRotator` 0.0 0.0 (`KismetMathLibrary.Lerp` 0.0 (select `bool` (>= (`self.Dot Product`) 0.0) :`false` -90.0 :`true` 90.0 :!type "Float (single-precision)") _alpha)) false false)))
    (else
      (set `self.PortaAberta` true)
      (set `self.Dot Product` (`KismetMathLibrary.Dot_VectorVector` (`KismetMathLibrary.Normal` (- (`self.K2_GetActorLocation` self) (`self.K2_GetActorLocation` (`self.Player Ref`)))) (`self.GetActorForwardVector` self)))
      (goto _label :!via `PlayFromStart`))))

(fn `UserConstructionScript`
  (`parent.UserConstructionScript`))