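; Locker hide spot that extends a hide-actor parent with an animated swinging door.
; Interact, gated by CanInteract, swings the door mesh open on a timeline, then hands off to the parent's Interact.
; The parent's FinishMovingED dispatcher, bound on BeginPlay, triggers the closing timeline, which re-enables interaction when it finishes.
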(event `self.ReceiveBeginPlay`
  (`parent.ReceiveBeginPlay`)
  (add `self.FinishMovingED` (delegate `FinishMovingED_Event_0`)))

(event `FinishMovingED_Event_0`
  (`self.Close_Door`))

(event `/Game/BP/Interface/BPI_Interaction.Interact`
  (if (`self.CanInteract`)
    (set `self.CanInteract` false)
    (bind (_direction _alpha) (`Timeline|OpenLockerDoor` :!via `PlayFromStart`)
      (:`Update`
        (`SceneComponent.K2_SetRelativeRotation` (`self.StaticMesh1`) (`KismetMathLibrary.MakeRotator` 0.0 0.0 (`KismetMathLibrary.Lerp` 0.0 90.0 _alpha)) false false))
      (:`Finished`
        (`parent.Interact`)))))

(event `Close_Door`
  (bind (_direction _alpha) (`Timeline|CloseLockDoor` :!via `PlayFromStart`)
    (:`Update`
      (`SceneComponent.K2_SetRelativeRotation` (`self.StaticMesh1`) (`KismetMathLibrary.MakeRotator` 0.0 0.0 (`KismetMathLibrary.Lerp` 90.0 0.0 _alpha)) false false))
    (:`Finished`
      (set `self.CanInteract` true))))

(fn `UserConstructionScript`
  (`parent.UserConstructionScript`))