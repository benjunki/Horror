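; Hiding spot actor that moves the player character into or out of hiding when interacted with.
; Entering disables player collision, movement and inventory opening; all three are restored once the exit move finishes.
; A looping frame-delta timer stands in for Tick, sliding the player at constant speed toward the HidingPosition or ExitPosition component.
; On arrival it clears the timers, fires the FinishMoving dispatcher and flips the player's IsHiding flag.
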(event `self.ReceiveBeginPlay`
  (bind _asl1_horror_character (cast `/Game/GameBP/Level1/L1_Horror_Character` (`GameplayStatics.GetPlayerCharacter` 0)))
  (set `self.Player Ref` _asl1_horror_character)
  (bind _ashorror_player_controller (cast `/Game/GameBP/Horror_PlayerController` (`GameplayStatics.GetPlayerController` 0)))
  (set `self.Controller Ref` _ashorror_player_controller))

(event `/Game/BP/Interface/BPI_Interaction.Interact`
  (bind _player_ref (`self.Player Ref`))
  (if (`/Game/GameBP/Level1/L1_Horror_Character.IsHiding` (`self.Player Ref`))
    (bind _returnvalue (`KismetSystemLibrary.K2_SetTimerDelegate` (delegate `MoveCharacter`) (`GameplayStatics.GetWorldDeltaSeconds`) true))
    (else
      (`self.SetActorEnableCollision` _player_ref false)
      (`CharacterMovementComponent.DisableMovement` (`Character.CharacterMovement` _player_ref))
      (set `/Game/GameBP/Horror_PlayerController.CanOpenIventory` false (`self.Controller Ref`))
      (bind _returnvalue_2 (`KismetSystemLibrary.K2_SetTimerDelegate` (delegate `MoveCharacter`) (`GameplayStatics.GetWorldDeltaSeconds`) true)))))

(event `MoveCharacter`
  (bind _player_ref (`self.Player Ref`))
  (`self.K2_SetActorTransform` _player_ref (`KismetMathLibrary.MakeTransform` (`KismetMathLibrary.VInterpTo_Constant` (`self.K2_GetActorLocation` _player_ref) (`SceneComponent.K2_GetComponentLocation` (select `bool` (`/Game/GameBP/Level1/L1_Horror_Character.IsHiding` (`self.Player Ref`)) :`false` (`self.HidingPosition`) :`true` (`self.ExitPosition`) :!type "SceneComponent Object Reference")) (`GameplayStatics.GetWorldDeltaSeconds`) 1000.0)) false false)
  (if (== (`self.K2_GetActorLocation` (`self.Player Ref`)) (`SceneComponent.K2_GetComponentLocation` (select `bool` (`/Game/GameBP/Level1/L1_Horror_Character.IsHiding` (`self.Player Ref`)) :`false` (`self.HidingPosition`) :`true` (`self.ExitPosition`) :!type "SceneComponent Object Reference")) :`ErrorTolerance` 0.1)
    (`KismetSystemLibrary.K2_ClearAndInvalidateTimerHandle` (stale `/Game/BP/Interface/BPI_Interaction.Interact` _returnvalue_2))
    (`KismetSystemLibrary.K2_ClearAndInvalidateTimerHandle` (stale `/Game/BP/Interface/BPI_Interaction.Interact` _returnvalue))
    (`self.FinishingMoving`)))

(event `FinishingMoving`
  (bind _player_ref (`self.Player Ref`))
  (bind _player_ref_2 (`self.Player Ref`))
  (`self.FinishMovingED`)
  (if (`/Game/GameBP/Level1/L1_Horror_Character.IsHiding` _player_ref)
    (set `/Game/GameBP/Level1/L1_Horror_Character.IsHiding` false _player_ref)
    (`self.SetActorEnableCollision` _player_ref_2 true)
    (`CharacterMovementComponent.SetMovementMode` (`Character.CharacterMovement` _player_ref_2) "MOVE_Walking" 0)
    (set `/Game/GameBP/Horror_PlayerController.CanOpenIventory` true (`self.Controller Ref`))
    (else
      (set `/Game/GameBP/Level1/L1_Horror_Character.IsHiding` true _player_ref))))

(fn `UserConstructionScript`)